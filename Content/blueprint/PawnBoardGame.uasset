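; Board game pawn that manages a list of players and which one is currently selected.
; BeginPlay spawns two Player actors with different starting money and stores them in the Players array.
; ChangePlayer swaps the viewport to the chosen player's Screen widget, with Q and E jumping to the first and second player.
; NextPlayer advances the selection and wraps to the first, though nothing in this Blueprint calls it.
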(event EventBeginPlay
  (bind _returnvalue (Game|SpawnActorfromClass "/Game/Player.Player_C" (Math|Transform|MakeTransform "0, 0, 0") false 0))
  (Variables|/Game/Player.Player_C|Setmoney _returnvalue 100)
  (Utilities|Array|Add (Variables|Default|Getplayers) _returnvalue)
  (bind _returnvalue_2 (Game|SpawnActorfromClass "/Game/Player.Player_C" (Math|Transform|MakeTransform "0, 0, 0") false 0))
  (Variables|/Game/Player.Player_C|Setmoney _returnvalue_2 222)
  (Utilities|Array|Add (Variables|Default|Getplayers) _returnvalue_2))

(event EventActorBeginOverlap
  (params (OtherActor :type Actor%20Object%20Reference)))

(event EventTick
  (params (DeltaSeconds :type Float%20%28single-precision%29)))

(event Input|KeyboardEvents|E
  (:Pressed
    (CallFunction|ChangePlayer 1)))

(event Input|KeyboardEvents|Q
  (:Pressed
    (CallFunction|ChangePlayer)))

(fn ConstructionScript)

(fn ChangePlayer
  (params (index :type Integer))
  (Widget|RemovefromParent (Variables|/Game/Player.Player_C|Getscreen (Variables|Default|GetselectPlayer)))
  (bind _output_get (Variables|Default|SetselectPlayer (Utilities|Array|Get(acopy) (Variables|Default|Getplayers) index)))
  (UserInterface|Viewport|AddtoViewport (Variables|/Game/Player.Player_C|Getscreen _output_get) 0))

(fn NextPlayer
  (bind _players (Variables|Default|Getplayers))
  (bind _selectplayer (Variables|Default|GetselectPlayer))
  (bind _returnvalue (Utilities|Array|FindItem _players _selectplayer))
  (if (== (Utilities|Array|LastIndex _players) _returnvalue)
    (CallFunction|ChangePlayer)
    (else
      (CallFunction|ChangePlayer (+ _returnvalue 1)))))